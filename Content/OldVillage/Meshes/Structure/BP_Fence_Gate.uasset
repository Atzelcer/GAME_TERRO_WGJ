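; BP_Fence_Gate is an Old Village fence gate prop, configured entirely in its construction script.
; A GateStyle setting swaps static meshes: Flat and Rounded set the gate, Sloped sets only the pole, and Mixed randomizes both.
; A clamped open-to-closed slider lerps a yaw that is added to the gate's local rotation.
; Its event graph holds only disabled stubs, so it has no runtime logic.
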(fn `UserConstructionScript`
  (bind _gate (`self.gate`))
  (switch `/Game/OldVillage/Meshes/Structure/Enumerators/BP_Fence_Enum` (`self.Gate Style`)
    (:`NewEnumerator0`
      (`StaticMeshComponent.SetStaticMesh` (`self.gate`) "/Game/OldVillage/Meshes/Structure_Components/SM_Fence_Flat_Gate_001.SM_Fence_Flat_Gate_001"))
    (:`NewEnumerator1`
      (`StaticMeshComponent.SetStaticMesh` (`self.gate`) "/Game/OldVillage/Meshes/Structure_Components/SM_Fence_Rounded_Gate_001.SM_Fence_Rounded_Gate_001"))
    (:`NewEnumerator2`
      (`StaticMeshComponent.SetStaticMesh` (`self.gate_pole`) "/Game/OldVillage/Meshes/Structure_Components/SM_Fence_gate_pole_002.SM_Fence_gate_pole_002"))
    (:`NewEnumerator3`
      (switch `int` (`KismetMathLibrary.RandomInteger` 2)
        (:`0`
          (`StaticMeshComponent.SetStaticMesh` (`self.gate_pole`) "/Game/OldVillage/Meshes/Structure_Components/SM_Fence_gate_pole_002.SM_Fence_gate_pole_002"))
        (:`1`
          _))
      (switch `int` (`KismetMathLibrary.RandomInteger` 3)
        (:`0`
          (`StaticMeshComponent.SetStaticMesh` _gate "/Game/OldVillage/Meshes/Structure_Components/SM_Fence_Sloped_Gate_001.SM_Fence_Sloped_Gate_001"))
        (:`1`
          (`StaticMeshComponent.SetStaticMesh` _gate "/Game/OldVillage/Meshes/Structure_Components/SM_Fence_Rounded_Gate_001.SM_Fence_Rounded_Gate_001"))
        (:`2`
          (`StaticMeshComponent.SetStaticMesh` _gate "/Game/OldVillage/Meshes/Structure_Components/SM_Fence_Flat_Gate_001.SM_Fence_Flat_Gate_001")))))
  (`SceneComponent.K2_AddLocalRotation` (`self.gate`) (`KismetMathLibrary.RLerp` (`KismetMathLibrary.MakeRotator` 0.0 0.0 0.0) (`KismetMathLibrary.MakeRotator` 0.0 0.0 -170.0) (`KismetMathLibrary.FClamp` (`self.Gate Rotation 1= Open 0= Closed`))) false false))