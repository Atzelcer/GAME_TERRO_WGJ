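; Modular 1m x 2m Old Village wall piece, configured entirely in the construction script; event graph is unused.
; ChooseComponent and AbbandonedBuilding select basic, corner or bend meshes and their offsets; non-abandoned Basic Wall keeps the component's existing mesh.
; Interior and exterior material overrides fill two slots, with a dynamic instance tinting exterior stucco via StuccoColor.
; Bend swaps those slots and builds its tinted instance from a hardcoded stone-to-stucco material.
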(fn `UserConstructionScript`
  (bind _static_mesh (`self.Static Mesh`))
  (bind _static_mesh_2 (`self.Static Mesh`))
  (bind _static_mesh_3 (`self.Static Mesh`))
  (bind _static_mesh_4 (`self.Static Mesh`))
  (bind _static_mesh_5 (`self.Static Mesh`))
  (bind _static_mesh_6 (`self.Static Mesh`))
  (bind _static_mesh_7 (`self.Static Mesh`))
  (bind _static_mesh_8 (`self.Static Mesh`))
  (bind _static_mesh_9 (`self.Static Mesh`))
  (bind _static_mesh_10 (`self.Static Mesh`))
  (bind _exterior_material_override (`self.Exterior Material Override`))
  (bind _static_mesh_11 (`self.Static Mesh`))
  (`PrimitiveComponent.SetMaterial` (`self.Static Mesh`) 0 (`self.Interior Material Override`))
  (`PrimitiveComponent.SetMaterial` (`self.Static Mesh`) 1 _exterior_material_override)
  ;[1 1 1] Change stucco Color
  (bind _returnvalue (`PrimitiveComponent.CreateDynamicMaterialInstance` (`self.Static Mesh`) 1 _exterior_material_override))
  (`MaterialInstanceDynamic.SetVectorParameterValue` _returnvalue "Material 2 Color multiplier" (`self.Stucco Color`))
  (switch `/Game/OldVillage/Meshes/Structure/Enumerators/BP_1mx2m_enum` (`self.Choose component`)
    (:`NewEnumerator0`
      ;[1 1 1] Basic Wall
      (if (`self.Abbandoned Building`)
        (`StaticMeshComponent.SetStaticMesh` _static_mesh_11 "/Game/OldVillage/Meshes/Structure_Components/SM_Wall_1mx2m_Edge_L_001_abbandoned.SM_Wall_1mx2m_Edge_L_001_abbandoned")
        (`SceneComponent.K2_SetRelativeTransform` _static_mesh_11 (`KismetMathLibrary.MakeTransform` (0.0 0.0 0.0) (struct) (1.0 1.0 1.0)) false false)))
    (:`NewEnumerator1`
      (if (`self.Abbandoned Building`)
        ;[1 1 1] Corner 90 IN R
        (`StaticMeshComponent.SetStaticMesh` _static_mesh_6 "/Game/OldVillage/Meshes/Structure_Components/SM_Wall_1mx2m_Edge_L_001_abbandoned.SM_Wall_1mx2m_Edge_L_001_abbandoned")
        (`SceneComponent.K2_SetRelativeTransform` _static_mesh_6 (`KismetMathLibrary.MakeTransform` (0.0 0.0 0.0) (struct) (1.0 1.0 1.0)) false false)
        (else
          (`StaticMeshComponent.SetStaticMesh` _static_mesh_5 "/Game/OldVillage/Meshes/Structure_Components/SM_Wall_1mx2m_Edge_L_001.SM_Wall_1mx2m_Edge_L_001")
          (`SceneComponent.K2_SetRelativeTransform` _static_mesh_5 (`KismetMathLibrary.MakeTransform` (0.0 0.0 0.0) (struct) (1.0 1.0 1.0)) false false))))
    (:`NewEnumerator7`
      (if (`self.Abbandoned Building`)
        ;[1 1 1] Corner 90 OUT R
        (`StaticMeshComponent.SetStaticMesh` _static_mesh_4 "/Game/OldVillage/Meshes/Structure_Components/SM_Wall_1mx2m_Edge_Out_R_001_abbandoned.SM_Wall_1mx2m_Edge_Out_R_001_abbandoned")
        (`SceneComponent.K2_SetRelativeTransform` _static_mesh_4 (`KismetMathLibrary.MakeTransform` (0.0 0.0 0.0) (struct) (1.0 1.0 1.0)) false false)
        (else
          (`StaticMeshComponent.SetStaticMesh` _static_mesh_3 "/Game/OldVillage/Meshes/Structure_Components/SM_Wall_1mx2m_Edge_Out_R_001.SM_Wall_1mx2m_Edge_Out_R_001")
          (`SceneComponent.K2_SetRelativeTransform` _static_mesh_3 (`KismetMathLibrary.MakeTransform` (0.0 0.0 0.0) (struct) (1.0 1.0 1.0)) false false))))
    (:`NewEnumerator2`
      (if (`self.Abbandoned Building`)
        ;[1 1 1] Corner 90 IN L
        (`StaticMeshComponent.SetStaticMesh` _static_mesh_2 "/Game/OldVillage/Meshes/Structure_Components/SM_Wall_1mx2m_Edge_R_001_abbandoned.SM_Wall_1mx2m_Edge_R_001_abbandoned")
        (`SceneComponent.K2_SetRelativeTransform` _static_mesh_2 (`KismetMathLibrary.MakeTransform` (100.0 0.0 0.0) (struct) (1.0 1.0 1.0)) false false)
        (else
          (`StaticMeshComponent.SetStaticMesh` _static_mesh "/Game/OldVillage/Meshes/Structure_Components/SM_Wall_1mx2m_Edge_R_001.SM_Wall_1mx2m_Edge_R_001")
          (`SceneComponent.K2_SetRelativeTransform` _static_mesh (`KismetMathLibrary.MakeTransform` (100.0 0.0 0.0) (struct) (1.0 1.0 1.0)) false false))))
    (:`NewEnumerator8`
      (if (`self.Abbandoned Building`)
        ;[1 1 1] Corner 90 OUT L
        (`StaticMeshComponent.SetStaticMesh` _static_mesh_10 "/Game/OldVillage/Meshes/Structure_Components/SM_Wall_1mx2m_Edge_Out_L_001_abbandoned.SM_Wall_1mx2m_Edge_Out_L_001_abbandoned")
        (`SceneComponent.K2_SetRelativeTransform` _static_mesh_10 (`KismetMathLibrary.MakeTransform` (100.0 0.0 0.0) (struct) (1.0 1.0 1.0)) false false)
        (else
          (`StaticMeshComponent.SetStaticMesh` _static_mesh_9 "/Game/OldVillage/Meshes/Structure_Components/SM_Wall_1mx2m_Edge_Out_L_001.SM_Wall_1mx2m_Edge_Out_L_001")
          (`SceneComponent.K2_SetRelativeTransform` _static_mesh_9 (`KismetMathLibrary.MakeTransform` (100.0 0.0 0.0) (struct) (1.0 1.0 1.0)) false false))))
    (:`NewEnumerator9`
      (`PrimitiveComponent.SetMaterial` (`self.Static Mesh`) 1 (`self.Interior Material Override`))
      (`PrimitiveComponent.SetMaterial` (`self.Static Mesh`) 0 (`self.Exterior Material Override`))
      ;[1 1 1] Change stucco Color
      (bind _returnvalue_2 (`PrimitiveComponent.CreateDynamicMaterialInstance` (`self.Static Mesh`) 0 "/Game/OldVillage/Materials/Tileable/MI_Blend_Stones_Exterior_001_to_Stucco_fine_001_parallax.MI_Blend_Stones_Exterior_001_to_Stucco_fine_001_parallax"))
      (`MaterialInstanceDynamic.SetVectorParameterValue` _returnvalue_2 "Material 2 Color multiplier" (`self.Stucco Color`))
      (if (`self.Abbandoned Building`)
        ;[1 1 1] Bend
        (`StaticMeshComponent.SetStaticMesh` _static_mesh_8 "/Game/OldVillage/Meshes/Structure_Components/SM_Wall_1mx2m_Bend_001_Abbandoned.SM_Wall_1mx2m_Bend_001_Abbandoned")
        (`SceneComponent.K2_SetRelativeTransform` _static_mesh_8 (`KismetMathLibrary.MakeTransform` (0.0 0.0 0.0) (struct) (1.0 1.0 1.0)) false false)
        (else
          (`StaticMeshComponent.SetStaticMesh` _static_mesh_7 "/Game/OldVillage/Meshes/Structure_Components/SM_Wall_1mx2m_Bend_001.SM_Wall_1mx2m_Bend_001")
          (`SceneComponent.K2_SetRelativeTransform` _static_mesh_7 (`KismetMathLibrary.MakeTransform` (0.0 0.0 0.0) (struct) (1.0 1.0 1.0)) false false))))))