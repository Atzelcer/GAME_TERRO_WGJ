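; Configurable structural pole prop for the Old Village set, built entirely in the Construction Script with no runtime logic.
; ChooseComponent selects one of three pole types, while the AbbandonedBuilding and SimplePole flags swap in abandoned or simplified meshes.
; Pole 02 also resets the mesh's relative transform to adjust its orientation.
; A final world-scale step combines Scale, per-axis X/Y adjustments and Lenght on Z, overriding any branch-set scale.
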(fn `UserConstructionScript`
  (bind _static_mesh (`self.Static Mesh`))
  (bind _static_mesh_2 (`self.Static Mesh`))
  (bind _static_mesh_3 (`self.Static Mesh`))
  (bind _scale (`self.Scale`))
  (bind _static_mesh_4 (`self.Static Mesh`))
  (switch `/Game/OldVillage/Meshes/Structure/Enumerators/BP_Pole_Enum` (`self.Choose component`)
    (:`NewEnumerator0`
      ;[1 1 1] Pole 01
      (if (`self.Abbandoned Building`)
        (`StaticMeshComponent.SetStaticMesh` (`self.Static Mesh`) "/Game/OldVillage/Meshes/Structure_Components/SM_Pole_001_abbandoned.SM_Pole_001_abbandoned")
        (if (`self.Simple pole`)
          (`StaticMeshComponent.SetStaticMesh` (`self.Static Mesh`) "/Game/OldVillage/Meshes/Structure_Components/SM_Pole_001_simple_abbandoned.SM_Pole_001_simple_abbandoned"))
        (elif (`self.Simple pole`)
          (`StaticMeshComponent.SetStaticMesh` (`self.Static Mesh`) "/Game/OldVillage/Meshes/Structure_Components/SM_Pole_001_simple.SM_Pole_001_simple"))))
    (:`NewEnumerator1`
      ;[1 1 1] Pole 02
      (if (`self.Abbandoned Building`)
        (`StaticMeshComponent.SetStaticMesh` _static_mesh_4 "/Game/OldVillage/Meshes/Structure_Components/SM_Pole_002_abbandoned.SM_Pole_002_abbandoned")
        (`SceneComponent.K2_SetRelativeTransform` _static_mesh_4 (`KismetMathLibrary.MakeTransform` (0.0 0.0 0.0) (struct :`Yaw` -90.0) (1.0 1.0 1.0)) false false)
        (if (`self.Simple pole`)
          (`StaticMeshComponent.SetStaticMesh` _static_mesh_3 "/Game/OldVillage/Meshes/Structure_Components/SM_Pole_001_simple_abbandoned.SM_Pole_001_simple_abbandoned")
          (`SceneComponent.K2_SetRelativeTransform` _static_mesh_3 (`KismetMathLibrary.MakeTransform` (0.0 0.0 0.0) (struct) (0.0 1.0 0.0)) false false))
        (else
          (`StaticMeshComponent.SetStaticMesh` _static_mesh "/Game/OldVillage/Meshes/Structure_Components/SM_Pole_002.SM_Pole_002")
          (`SceneComponent.K2_SetRelativeTransform` _static_mesh (`KismetMathLibrary.MakeTransform` (0.0 0.0 0.0) (struct :`Yaw` -90.0) (1.0 1.0 1.0)) false false)
          (if (`self.Simple pole`)
            (`StaticMeshComponent.SetStaticMesh` _static_mesh_2 "/Game/OldVillage/Meshes/Structure_Components/SM_Pole_001_simple.SM_Pole_001_simple")
            (`SceneComponent.K2_SetRelativeTransform` _static_mesh_2 (`KismetMathLibrary.MakeTransform` (0.0 0.0 0.0) (struct) (0.0 1.0 0.0)) false false)))))
    (:`NewEnumerator2`
      ;[1 1 1] Pole 03
      (if (`self.Abbandoned Building`)
        (`StaticMeshComponent.SetStaticMesh` (`self.Static Mesh`) "/Game/OldVillage/Meshes/Structure_Components/SM_Pole_003_abbandoned.SM_Pole_003_abbandoned")
        (if (`self.Simple pole`)
          (`StaticMeshComponent.SetStaticMesh` (`self.Static Mesh`) "/Game/OldVillage/Meshes/Structure_Components/SM_Pole_002_simple_abbandoned.SM_Pole_002_simple_abbandoned"))
        (else
          (`StaticMeshComponent.SetStaticMesh` (`self.Static Mesh`) "/Game/OldVillage/Meshes/Structure_Components/SM_Pole_003.SM_Pole_003")
          (if (`self.Simple pole`)
            (`StaticMeshComponent.SetStaticMesh` (`self.Static Mesh`) "/Game/OldVillage/Meshes/Structure_Components/SM_Pole_002_simple.SM_Pole_002_simple"))))))
  ;[1 1 1] Set lenght and Scale
  (`SceneComponent.SetWorldScale3D` (`self.Static Mesh`) (`KismetMathLibrary.MakeVector` (+ _scale (`self.Scale adjust X`)) (+ _scale (`self.Scale adjust Y`)) (+ _scale (`self.Lenght`)))))